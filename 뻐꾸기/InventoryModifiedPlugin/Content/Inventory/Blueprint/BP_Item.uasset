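; BP_Item is a world inventory item that a Character picks up by overlapping it.
; On BeginPlay it sets its mesh from its data table row.
; On overlap it finds the BP_InventoryData actor whose Index matches the player controller ID, passes it the row's item data and, if the row is found, destroys itself.
; A drop event rebuilds its DT_Item row reference and mesh from an indexed entry in the owner inventory.
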(event Custom|EventDropItem
  (params (ItemIndex :type Integer))
  (CallFunction|SetItemData ItemIndex))

(event EventBeginPlay
  (bind _itemslotdata (Variables|Default|GetItemSlotData))
  (bind _returnvalue (Utilities|GetDataTableRow (.datatable (.item _itemslotdata)) (.rowname (.item _itemslotdata)))
    (:then
      (Components|StaticMesh|SetStaticMesh (Variables|Default|GetStaticMesh) (.Static_Mesh (Utilities|Struct|BreakS_Item _returnvalue))))))

(event Collision|EventActorBeginOverlap
  (params (OtherActor :type Actor%20Object%20Reference))
  (bind _itemslotdata (Variables|Default|GetItemSlotData))
  ;[0 0.04667 1] Take Item. Player state로부터 index를 받아와야함
  (bind _ascharacter (Utilities|Casting|CastToCharacter OtherActor))
  (bind _outactors (Actor|GetAllActorsOfClass "/InventoryModifiedPlugin/Inventory/Blueprint/BP_InventoryData.BP_InventoryData_C"))
  (for _array_element _outactors
    (if (== (Variables|/InventoryModifiedPlugin/Inventory/Blueprint/BP_InventoryData.BP_InventoryData_C|GetIndex _array_element) (Class|GameplayStatics|GetPlayerControllerID (Game|GetPlayerController (Variables|/Script/Engine.Pawn|GetPlayerState _ascharacter))))
      (Variables|Default|SetOwnerInventory _array_element)
      (bind _returnvalue (Utilities|GetDataTableRow (.datatable (.item _itemslotdata)) (.rowname (.item _itemslotdata)))
        (:then
          (Class|BPItemDataInterface|TakeItemData(Message) (Variables|Default|GetOwnerInventory) (Utilities|Struct|MakeS_Inventory (.Name (Utilities|Struct|BreakS_Item _returnvalue)) (.Icon (Utilities|Struct|BreakS_Item _returnvalue)) (.Static_Mesh (Utilities|Struct|BreakS_Item _returnvalue)) (.Type (Utilities|Struct|BreakS_Item _returnvalue)) (.InventoryIndex (Utilities|Struct|BreakS_Item _returnvalue)) (.ItemIndex (Utilities|Struct|BreakS_Item _returnvalue))))
          (Actor|DestroyActor))))))

(fn ConstructionScript)

(fn SetItemData
  (params (ItemIndex :type Integer%20%28by%20ref%29))
  (bind _ownerinventory (Variables|Default|GetOwnerInventory))
  (bind _inventorydata (Variables|/InventoryModifiedPlugin/Inventory/Blueprint/BP_InventoryData.BP_InventoryData_C|GetInventoryData _ownerinventory))
  (bind _output (Utilities|Array|Get(acopy) _inventorydata ItemIndex))
  (bind (_name _icon _static_mesh) (Utilities|Struct|BreakS_Inventory _output))
  (Variables|Default|SetItemSlotData (Utilities|Struct|MakeS_Slots (Utilities|Struct|MakeDataTableRowHandle "/InventoryModifiedPlugin/Inventory/Blueprint/DT_Item.DT_Item" (Utilities|String|StringToName _name))))
  (Components|StaticMesh|SetStaticMesh (Variables|Default|GetStaticMesh) _static_mesh))