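; BP_Tower is a tower that periodically fires a hitscan shot toward a target location and damages whatever it hits.
; The construction script stores EnemyLocation from the last BP_TowerAgainstTarget found, so the aim point is not updated during play.
; Tick uses a five-second Delay as a fire timer, then line-traces from the Muzzle socket with debug drawing, spawns a muzzle particle and applies damage to the hit actor.
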(event EventBeginPlay)

(event Collision|EventActorBeginOverlap
  (params (OtherActor :type Actor%20Object%20Reference)))

(event EventTick
  (params (DeltaSeconds :type Float%20%28single-precision%29))
  (|CallParentFunction DeltaSeconds)
  (Utilities|FlowControl|Delay 5.0)
  (bind _outhit (Collision|LineTraceByChannel (Transformation|GetSocketLocation (Variables|Default|GetStaticMesh) "Muzzle") (Variables|Default|GetEnemyLocation) "TraceTypeQuery1" false 0 "ForDuration"))
  (Effects|SpawnEmitteratLocation "/Engine/Tutorial/SubEditors/TutorialAssets/TutorialParticleSystem.TutorialParticleSystem" (Transformation|GetSocketLocation (Variables|Default|GetStaticMesh) "Muzzle"))
  (Game|Damage|ApplyDamage (.HitActor (Collision|BreakHitResult _outhit)) 5e+01 0 0))

(fn ConstructionScript
  (|CallParentFunction)
  (bind _outactors (Actor|GetAllActorsOfClass "/InventoryModifiedPlugin/Inventory/Blueprint/BP_TowerAgainstTarget.BP_TowerAgainstTarget_C"))
  (for _array_element _outactors
    (Variables|Default|SetEnemyLocation (Transformation|GetActorLocation _array_element))))