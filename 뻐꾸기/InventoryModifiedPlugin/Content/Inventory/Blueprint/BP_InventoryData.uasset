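; Inventory data actor that stores inventory and equipment arrays and handles item pickup, drop, monster-loot spawning and use.
; Drops spawn BP_Item; loot is briefly appended to the inventory to pass an index, then removed.
; Use looks up DT_Item by name and switches on type: gear swaps into a fixed equipment slot, potions add HP or MP on BP_ItemPS, and Tower items spawn BP_Tower ahead of the player.
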(event Custom|EventSpawnItem
  (params (ItemData :type S%20Item%20Structure) (Spawn%20Transform%20Location :type Vector))
  (bind (_name _damage _requiredlevel _icon _static_mesh _type _inventoryindex _itemindex) (Utilities|Struct|BreakS_Item ItemData))
  ;[1 0 0] 몬스터를 잡고 아이템 드롭하는 기능.소환할 Location과 Item을 입력해야함.
  (bind _newparam (CallFunction|FnTakeItemData (Utilities|Struct|MakeS_Inventory _name _icon _static_mesh _type _inventoryindex _itemindex)))
  (bind _returnvalue (Game|SpawnActorfromClass :Class "/InventoryModifiedPlugin/Inventory/Blueprint/BP_Item.BP_Item_C" :SpawnTransform (Math|Transform|MakeTransform Spawn%20Transform%20Location "0, 0, 0" "1.000000,1.000000,1.000000") :CollisionHandlingOverride "AdjustIfPossibleButAlwaysSpawn" :TransformScaleMethod "MultiplyWithRoot" :Instigator 0))
  (Default|EventDropItem _returnvalue _newparam)
  (Utilities|Array|RemoveIndex (Variables|Default|GetInventoryData) _newparam))

(event EventUseItemData
  (params (ItemIndex :type Integer))
  (bind _returnvalue (Game|GetPlayerCharacter 0))
  (bind _returnvalue_2 (Transformation|GetActorForwardVector _returnvalue))
  (bind _returnvalue_3 (Transformation|GetActorLocation _returnvalue))
  (bind _returnvalue_4 (* _returnvalue_2 "500.000000,500.000000,0.000000"))
  (bind _returnvalue_5 (+ _returnvalue_3 _returnvalue_4))
  (bind _returnvalue_6 (Utilities|GetDataTableRow "/InventoryModifiedPlugin/Inventory/Blueprint/DT_Item.DT_Item" (Utilities|String|StringToName (.Name (Utilities|Struct|BreakS_Inventory (Utilities|Array|Get(acopy) (Variables|Default|GetInventoryData) ItemIndex)))))
    (:then
      (switch Utilities|FlowControl|Switch|SwitchonE_Item_Types (.Type (Utilities|Struct|BreakS_Item _returnvalue_6))
        (:NewEnumerator0
          (Development|PrintString "공격 아이템 장비" :!label _label)
          (CallFunction|SwapInventoryandEquipment ItemIndex))
        (:NewEnumerator1
          (goto _label))
        (:NewEnumerator2
          (goto _label))
        (:NewEnumerator3
          (goto _label))
        (:NewEnumerator4
          (Development|PrintString "아머 아이템 장비")
          (CallFunction|SwapInventoryandEquipment ItemIndex 1))
        (:NewEnumerator5
          (Development|PrintString "책 아이템 장비")
          (CallFunction|SwapInventoryandEquipment ItemIndex 4))
        (:NewEnumerator6
          (Development|PrintString "목걸이 아이템 장비")
          (CallFunction|SwapInventoryandEquipment ItemIndex 3))
        (:NewEnumerator7
          (Development|PrintString "반지 아이템 장비")
          (CallFunction|SwapInventoryandEquipment ItemIndex 2))
        (:NewEnumerator8
          (Development|PrintString "힐링 아이템 사용")
          (bind _returnvalue_7 (Utilities|GetDataTableRow "/InventoryModifiedPlugin/Inventory/Blueprint/DT_Item.DT_Item" (Utilities|String|StringToName (.name (Utilities|Array|Get(acopy) (Variables|Default|GetInventoryData) ItemIndex))))
            (:then
              (bind _asbp_item_ps (Utilities|Casting|CastToBP_ItemPS (Game|GetPlayerState 0)))
              (Variables|/InventoryModifiedPlugin/Inventory/Blueprint/BP_ItemPS.BP_ItemPS_C|SetHP _asbp_item_ps (+ (.heal _returnvalue_7) (Variables|/InventoryModifiedPlugin/Inventory/Blueprint/BP_ItemPS.BP_ItemPS_C|GetHP _asbp_item_ps)))
              (Utilities|Array|RemoveIndex (Variables|Default|GetInventoryData) ItemIndex))))
        (:NewEnumerator10
          (Development|PrintString "타워 아이템 사용")
          (Game|SpawnActorfromClass "/InventoryModifiedPlugin/Inventory/Blueprint/BP_Tower.BP_Tower_C" (Math|Transform|MakeTransform (Math|Vector|MakeVector (.x _returnvalue_5) (.y _returnvalue_5) 0.0) "0, 0, 0" "1.000000,1.000000,1.000000") "AdjustIfPossibleButAlwaysSpawn" "MultiplyWithRoot" 0 0)
          (Utilities|Array|RemoveIndex (Variables|Default|GetInventoryData) ItemIndex))
        (:NewEnumerator12
          (Development|PrintString "마나 아이템 사용")
          (bind _returnvalue_8 (Utilities|GetDataTableRow "/InventoryModifiedPlugin/Inventory/Blueprint/DT_Item.DT_Item" (Utilities|String|StringToName (.name (Utilities|Array|Get(acopy) (Variables|Default|GetInventoryData) ItemIndex))))
            (:then
              (bind _asbp_item_ps_2 (Utilities|Casting|CastToBP_ItemPS (Game|GetPlayerState 0)))
              (Variables|/InventoryModifiedPlugin/Inventory/Blueprint/BP_ItemPS.BP_ItemPS_C|SetMP _asbp_item_ps_2 (+ (.mana _returnvalue_8) (Variables|/InventoryModifiedPlugin/Inventory/Blueprint/BP_ItemPS.BP_ItemPS_C|GetMP _asbp_item_ps_2)))
              (Utilities|Array|RemoveIndex (Variables|Default|GetInventoryData) ItemIndex))))))))

(event EventBeginPlay
  (bind _asplayer_controller (Utilities|Casting|CastToPlayerController (Components|GetOwner)))
  (Variables|Default|SetIndex (Class|GameplayStatics|GetPlayerControllerID _asplayer_controller)))

(event EventTakeItemData
  (params (InventoryData :type S%20Inventory%20Structure))
  ;[1 1 1] Weapon Data를 인터페이스를 통해 받아오는 로직
  (CallFunction|FnTakeItemData InventoryData))

(event EventDropItemData
  (params (ItemIndex :type Integer))
  (bind _returnvalue (Game|Player|GetPlayerPawn 0))
  (bind _returnvalue_2 (Transformation|GetActorLocation _returnvalue))
  (bind _returnvalue_3 (Game|SpawnActorfromClass :Class "/InventoryModifiedPlugin/Inventory/Blueprint/BP_Item.BP_Item_C" :SpawnTransform (Math|Transform|MakeTransform (Math|Vector|MakeVector (+ (.x _returnvalue_2) (Math|Random|RandomFloatinRange -1e+02 1e+02)) (+ (.y _returnvalue_2) (Math|Random|RandomFloatinRange -1e+02 1e+02)) (+ (.z _returnvalue_2) 1e+02)) "0, 0, 0" "1.000000,1.000000,1.000000") :CollisionHandlingOverride "AdjustIfPossibleButAlwaysSpawn" :TransformScaleMethod "MultiplyWithRoot" :Instigator 0))
  (Default|EventDropItem _returnvalue_3 ItemIndex)
  (Utilities|Array|RemoveIndex (Variables|Default|GetInventoryData) ItemIndex))

(fn ConstructionScript
  (bind _foundwidgets (Widget|GetAllWidgetsOfClass "/InventoryModifiedPlugin/Inventory/Widget/WBP_Inventory.WBP_Inventory_C" true))
  (for _array_element _foundwidgets
    (Variables|Default|SetWBP_InventoryRef _array_element)))

(fn SwapInventoryandEquipment
  (params (InventoryIndex :type Integer) (EquipmentIndex :type Integer))
  (bind _equipmentdata (Variables|Default|GetEquipmentData))
  (bind _inventorydata (Variables|Default|GetInventoryData))
  (bind _output (Utilities|Array|Get(acopy) _inventorydata InventoryIndex))
  (bind _output_2 (Utilities|Array|Get(acopy) _equipmentdata EquipmentIndex))
  (bind _name (Utilities|Struct|BreakS_Inventory _output))
  (bind _returnvalue (Utilities|String|StringToName _name))
  (if (not (== _returnvalue "Item"))
    (if (not (== (Utilities|String|StringToName (.Name (Utilities|Struct|BreakS_Item _output_2))) "Item"))
      (LocalVariables|SetTmpEquipmentDataForSwap _output_2)
      (Utilities|FlowControl|Sequence
        (:then_0
          (bind _returnvalue_2 (Utilities|GetDataTableRow "/InventoryModifiedPlugin/Inventory/Blueprint/DT_Item.DT_Item" _returnvalue)
            (:then
              (Utilities|Array|Insert (Variables|Default|GetEquipmentData) _returnvalue_2 EquipmentIndex)
              (Utilities|Array|Insert (Variables|Default|GetInventoryData) (Utilities|Struct|MakeS_Inventory (.name (LocalVariables|GetTmpEquipmentDataForSwap)) (.icon (LocalVariables|GetTmpEquipmentDataForSwap)) (.static_mesh (LocalVariables|GetTmpEquipmentDataForSwap)) (.type (LocalVariables|GetTmpEquipmentDataForSwap)) (.inventoryindex (LocalVariables|GetTmpEquipmentDataForSwap)) (.itemindex (LocalVariables|GetTmpEquipmentDataForSwap))) InventoryIndex))))
        (:then_1
          (Utilities|Array|RemoveIndex _inventorydata (+ InventoryIndex 1))
          (Utilities|Array|RemoveIndex _equipmentdata (+ EquipmentIndex 1)))))))

(fn FnTakeItemData
  (params (StructRef :type S%20Inventory%20Structure%20%28by%20ref%29))
  (bind _structout (Utilities|Struct|SetmembersinS_Inventory StructRef (Utilities|Array|Length (Variables|Default|GetInventoryData))))
  (bind _returnvalue (Utilities|Array|Add (Variables|Default|GetInventoryData) _structout))
  (return _returnvalue))