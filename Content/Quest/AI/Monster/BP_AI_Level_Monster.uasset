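; Quest monster AI that chases the player and periodically attacks.
; From BeginPlay it runs AI MoveTo toward the player, restarting only on success.
; Tick feeds chained Delays that throttle turning toward the player and spawning BP_Attack at Arrow1's transform.
; A DropItem function, not called within this Blueprint, spawns a half-scale BP_CarryBox at the mesh location and prints a debug message.
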(event Custom|FollowActor
  ;[0 0 0] Move
  (AI|AIMoveTo self "0, 0, 0" (Game|GetPlayerCharacter 0) 1.5e+02 false
    (:OnSuccess
      (CallFunction|FollowActor))))

(event EventBeginPlay
  ;[0 0 0] Move
  (CallFunction|FollowActor))

(event EventTick
  (params (DeltaSeconds :type Float%20%28single-precision%29))
  ;[0 0 0] Attack
  (Utilities|FlowControl|Delay 0.5)
  (Transformation|SetActorRotation (Math|Rotator|FindLookatRotation (Transformation|GetWorldLocation (Variables|Character|GetArrow1)) (Transformation|GetActorLocation (Game|GetPlayerCharacter 0))))
  (Utilities|FlowControl|Delay 1.0)
  (Game|SpawnActorfromClass "/Game/Quest/AI/Monster/BP_Attack.BP_Attack_C" (Transformation|GetWorldTransform (Variables|Character|GetArrow1)) "AlwaysSpawn" "MultiplyWithRoot" 0 0))

(fn ConstructionScript)

(fn DropItem
  (Game|SpawnActorfromClass "/Game/Quest/Quest/BP_CarryBox.BP_CarryBox_C" (Math|Transform|MakeTransform (Transformation|GetWorldLocation (Variables|Character|GetMesh)) "0, 0, 0" "0.500000,0.500000,0.500000") "Undefined" "MultiplyWithRoot" 0 0)
  (Development|PrintString "drop item success"))