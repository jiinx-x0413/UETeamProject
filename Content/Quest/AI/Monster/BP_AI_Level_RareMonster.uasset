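; BP_AI_Level_RareMonster is a rare monster that chases the player and can drop a carry box.
; From BeginPlay it runs AI MoveTo toward player 0, restarting on each success, with no retry on failure.
; DropItem spawns a half-scale BP_CarryBox at the mesh's location and prints a debug message, but nothing in this Blueprint calls it.
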(event Custom|FollowActor
  ;[0 0 0] Move
  (AI|AIMoveTo self "0, 0, 0" (Game|GetPlayerCharacter 0) 1.5e+02 false
    (:OnSuccess
      (CallFunction|FollowActor))))

(event EventBeginPlay
  ;[0 0 0] Move
  (CallFunction|FollowActor))

(fn ConstructionScript)

(fn DropItem
  (Game|SpawnActorfromClass "/Game/Quest/Quest/BP_CarryBox.BP_CarryBox_C" (Math|Transform|MakeTransform (Transformation|GetWorldLocation (Variables|Character|GetMesh)) "0, 0, 0" "0.500000,0.500000,0.500000") "Undefined" "MultiplyWithRoot" 0 0)
  (Development|PrintString "drop item success"))