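; BP_Attack is a monster attack actor that explodes on contact with the player in the Quest game.
; When its StaticMesh overlaps a BP_Player_Quest, it spawns a half-scale explosion at the player, destroys itself and prints a debug damage message.
; No damage is applied; a comment only notes the intended HP function call.
; Tick runs a Delay that leads to nothing.
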(event OnComponentBeginOverlap(StaticMesh)
  (params (OverlappedComponent :type Primitive%20Component%20Object%20Reference) (OtherActor :type Actor%20Object%20Reference) (OtherComp :type Primitive%20Component%20Object%20Reference) (OtherBodyIndex :type Integer) (bFromSweep :type Boolean) (SweepResult :type Hit%20Result%20Structure%20%28by%20ref%29))
  ;[1 1 1] cast to bp_tp_character -> HP 바꾸는 함수 콜
  (bind _asbp_player_quest (Utilities|Casting|CastToBP_Player_Quest OtherActor))
  (Effects|SpawnEmitteratLocation "/Game/StarterContent/Particles/P_Explosion.P_Explosion" (Transformation|GetActorLocation _asbp_player_quest) "0, 0, 0" "0.500000,0.500000,0.500000")
  (Actor|DestroyActor)
  (Development|PrintString (Utilities|String|Append "damage : " (Utilities|String|ToString(Float) (Variables|Default|GetDamage)) " / 맞은넘 : " (Utilities|GetDisplayName 0))))

(event EventTick
  (params (DeltaSeconds :type Float%20%28single-precision%29))
  (Utilities|FlowControl|Delay 0.2))

(fn ConstructionScript)