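; BP_GM_Outgame is the game mode for the out-of-game levels: Menu, Lobby, Room and Result.
; On BeginPlay it switches on the current level name to create that level's UMG widget, store a reference and add it to the viewport.
; On the Result level it also reads win state, quest progress and player data from the BP_GI game instance and passes them to the result widget for display.
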(event EventBeginPlay
  (CallFunction|InitUI)
  (CallFunction|SetGameResult))

(fn ConstructionScript)

(fn InitUI
  (bind _returnvalue (Game|GetCurrentLevelName true))
  (switch string _returnvalue
    (:Menu
      (bind _returnvalue_2 (UserInterface|CreateWidget "/Game/Blueprints/UMG/UMG_Menu.UMG_Menu_C"))
      (bind _output_get (Variables|Reference|SetUIMenuRef _returnvalue_2))
      (UserInterface|Viewport|AddtoViewport _output_get 0))
    (:Lobby
      (bind _returnvalue_3 (UserInterface|CreateWidget "/Game/Blueprints/UMG/UMG_Lobby.UMG_Lobby_C"))
      (bind _output_get_2 (Variables|Reference|SetUILobbyRef _returnvalue_3))
      (UserInterface|Viewport|AddtoViewport _output_get_2 0))
    (:Room
      (bind _returnvalue_4 (UserInterface|CreateWidget "/Game/Blueprints/UMG/UMG_Room.UMG_Room_C"))
      (bind _output_get_3 (Variables|Reference|SetUIRoomRef _returnvalue_4))
      (UserInterface|Viewport|AddtoViewport _output_get_3 0))
    (:Result
      (bind _returnvalue_5 (UserInterface|CreateWidget "/Game/Blueprints/UMG/UMG_Result.UMG_Result_C"))
      (bind _output_get_4 (Variables|Reference|SetUIResultRef _returnvalue_5))
      (UserInterface|Viewport|AddtoViewport _output_get_4 0))))

(fn SetGameResult
  (bind _returnvalue (Game|GetCurrentLevelName true))
  (switch string _returnvalue
    (:Result
      ;[0 0 0] GI 데이터를 UI로 표시
      (bind _asbp_gi (Utilities|Casting|CastToBP_GI (Game|GetGameInstance)))
      (Variables|Reference|SetGIRef _asbp_gi)
      (Default|ShowGameResult (Variables|Reference|GetUIResultRef) (Variables|/Game/Blueprints/Gamemode/BP_GI.BP_GI_C|GetbIsWinGame (Variables|Reference|GetGIRef)) (Variables|/Game/Blueprints/Gamemode/BP_GI.BP_GI_C|GetE_Result (Variables|Reference|GetGIRef)))
      (Default|ShowQuestResult (Variables|Reference|GetUIResultRef) (Variables|/Game/Blueprints/Gamemode/BP_GI.BP_GI_C|GetMaxQuestStage (Variables|Reference|GetGIRef)) (Variables|/Game/Blueprints/Gamemode/BP_GI.BP_GI_C|GetLastQuestStage (Variables|Reference|GetGIRef)) (Variables|/Game/Blueprints/Gamemode/BP_GI.BP_GI_C|GetQuestMap (Variables|Reference|GetGIRef)))
      (Default|ShowPlayerResult (Variables|Reference|GetUIResultRef) (Variables|/Game/Blueprints/Gamemode/BP_GI.BP_GI_C|GetPlayerData (Variables|Reference|GetGIRef))))))