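; In-game GameMode that runs a staged quest match around a main tower, with a market and a win/lose ending.
; BeginPlay cross-links GameInstance, GameState, PlayerState and main UI, spawns the tower, and builds a quest-completion map from an enum.
; Callable functions spawn characters, start quests and spawn or destroy the market.
; EndGame evaluates stage-clear or stage-overrun from GameState, copies results to GameInstance, then opens the Result level.
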(event EventBeginPlay
  (Init|InitReference)
  (Init|InitUI)
  (RunGame|SpawnMainTower)
  (Init|InitStageandQuestVar))

(fn ConstructionScript)

(fn InitReference
  (Utilities|FlowControl|Sequence
    (:then_0
      (bind _asbp_gi (Utilities|Casting|CastToBP_GI (Game|GetGameInstance)))
      (bind _output_get (Variables|Reference|SetGIRef _asbp_gi))
      (Variables|/Game/Blueprints/Gamemode/BP_GI.BP_GI_C|SetGMIngameRef _output_get self))
    (:then_1
      (bind _asbp_gs (Utilities|Casting|CastToBP_GS (Game|GetGameState)))
      (bind _output_get_2 (Variables|Reference|SetGSRef _asbp_gs))
      (Variables|/Game/Blueprints/Gamemode/BP_GS.BP_GS_C|SetGMRef _output_get_2 self))
    (:then_2
      (bind _asbp_ps (Utilities|Casting|CastToBP_PS (Game|GetPlayerState 0)))
      (Variables|Reference|SetPSRef _asbp_ps))))

(fn InitUI
  (bind _returnvalue (UserInterface|CreateWidget "/Game/Blueprints/UMG/UMG_Game_Main.UMG_Game_Main_C"))
  (Variables|Reference|SetUIGameMainRef _returnvalue)
  (Utilities|FlowControl|Sequence
    (:then_0
      (UserInterface|Viewport|AddtoViewport (Variables|Reference|GetUIGameMainRef) 0))
    (:then_1
      (Variables|/Game/Blueprints/UMG/UMG_Game_Main.UMG_Game_Main_C|SetGMRef (Variables|Reference|GetUIGameMainRef) self))
    (:then_2
      (bind _output_get (Variables|/Game/Blueprints/UMG/UMG_Game_Main.UMG_Game_Main_C|SetGSRef (Variables|Reference|GetUIGameMainRef) (Variables|Reference|GetGSRef)))
      (Variables|/Game/Blueprints/Gamemode/BP_GS.BP_GS_C|SetUIGameMainRef _output_get (Variables|Reference|GetUIGameMainRef)))))

(fn SpawnMarket
  (Widget|SetVisibility (Variables|/Game/Blueprints/UMG/UMG_Game_Main.UMG_Game_Main_C|GetCP_MarketTime (Variables|Reference|GetUIGameMainRef)) "Visible")
  (bind _returnvalue (Game|SpawnActorfromClass "/Game/Blueprints/BP_Market_Sample.BP_Market_Sample_C" (Math|Transform|MakeTransform "0, 0, 0") "Undefined" "MultiplyWithRoot" 0 0))
  (Variables|Reference|SetMarket _returnvalue))

(fn DestroyMarket
  (Widget|SetVisibility (Variables|/Game/Blueprints/UMG/UMG_Game_Main.UMG_Game_Main_C|GetCP_MarketTime (Variables|Reference|GetUIGameMainRef)) "Hidden")
  (Utilities|IsValid (Variables|Reference|GetMarket)
    (:Is%20Valid
      (Actor|DestroyActor (Variables|Reference|GetMarket)))
    (:Is%20Not%20Valid
      (bind _outactors (Actor|GetAllActorsOfClass "/Game/Blueprints/BP_Market_Sample.BP_Market_Sample_C"))
      (for _array_element _outactors
        (Actor|DestroyActor _array_element)))))

(fn EndGame
  (ChangeGameState|WinGameClearStage)
  (ChangeGameState|LoseGameTimeover)
  (if (Variables|Result|GetbIsEndGame)
    ;[0 0 0] Set GameInstance
    (ChangeGameState|SetResultGI)
    ;[0 0 0] Level Transition :: Result
    (Game|OpenLevel(byName) "Result")))

(fn WinGameClearStage
  (if (Variables|/Game/Blueprints/Gamemode/BP_GS.BP_GS_C|GetIsStageCleared (Variables|Reference|GetGSRef))
    (Variables|Result|SetbIsEndGame true)
    (Variables|Result|SetbIsGameWin true)
    (Variables|Result|SetE_Result "NewEnumerator3")))

(fn LoseGameTimeover
  (bind _gsref (Variables|Reference|GetGSRef))
  (if (> (Variables|/Game/Blueprints/Gamemode/BP_GS.BP_GS_C|GetCurrentQuestStage _gsref) (Variables|/Game/Blueprints/Gamemode/BP_GS.BP_GS_C|GetMaxQuestStage _gsref))
    (Variables|Result|SetbIsEndGame true)
    (Variables|Result|SetbIsGameWin false)
    (Variables|Result|SetE_Result "NewEnumerator0")))

(fn SetResultGI
  ;[0 0 0] GameResult & Description
  (Variables|/Game/Blueprints/Gamemode/BP_GI.BP_GI_C|SetbIsWinGame (Variables|Reference|GetGIRef) (Variables|Result|GetbIsGameWin))
  (Variables|/Game/Blueprints/Gamemode/BP_GI.BP_GI_C|SetE_Result (Variables|Reference|GetGIRef) (Variables|Result|GetE_Result))
  ;[0 0 0] Quest
  (Variables|/Game/Blueprints/Gamemode/BP_GI.BP_GI_C|SetLastQuestStage (Variables|Reference|GetGIRef) (Variables|/Game/Blueprints/Gamemode/BP_GS.BP_GS_C|GetCurrentQuestStage (Variables|Reference|GetGSRef)))
  (Variables|/Game/Blueprints/Gamemode/BP_GI.BP_GI_C|SetQuestMap (Variables|Reference|GetGIRef) (Variables|/Game/Blueprints/Gamemode/BP_GS.BP_GS_C|GetQuestMap (Variables|Reference|GetGSRef))))

(fn InitStageandQuestVar
  (bind _output_get (Variables|Quest|SetMaxStage (|GetNumEnumEntries)))
  (bind _output_get_2 (Variables|/Game/Blueprints/Gamemode/BP_GS.BP_GS_C|SetMaxQuestStage (Variables|Reference|GetGSRef) _output_get))
  (Variables|/Game/Blueprints/Gamemode/BP_GI.BP_GI_C|SetMaxQuestStage (Variables|Reference|GetGIRef) _output_get_2)
  ;[0 0 0] Debug
  (Development|PrintString (Utilities|String|Append "MaxStage : " (Utilities|String|ToString(Integer) _output_get_2)))
  ;[0 0 0] Set QuestMap {QuestName : (bool) IsCompleted }
  (bind _enumvalue (|ForEachE_Quest_Sample)
    (:LoopBody
      (Utilities|Map|Add (Variables|Quest|GetQuestMap) (Utilities|String|EnumtoString _enumvalue) false))
    (:then
      (Variables|/Game/Blueprints/Gamemode/BP_GS.BP_GS_C|SetQuestMap (Variables|Reference|GetGSRef) (Variables|Quest|GetQuestMap))
      ;[0 0 0] Debug
      (bind _keys (Utilities|Map|Keys (Variables|Quest|GetQuestMap)))
      (for (_array_element _array_index) _keys
        (Development|PrintString (Utilities|String|Append "index : " (Utilities|String|ToString(Integer) _array_index) " / Key : " _array_element "/ Value : " (Utilities|String|ToString(Boolean) (.Value (Utilities|Map|Find (Variables|Quest|GetQuestMap) _array_element)))))))))

(fn SpawnMainTower
  (bind _returnvalue (Game|SpawnActorfromClass "/Game/Blueprints/BP_Tower_Sample.BP_Tower_Sample_C" (Math|Transform|MakeTransform "0, 0, 0") "Undefined" "MultiplyWithRoot" 0 0))
  (Variables|Reference|SetMainTower _returnvalue))

(fn SpawnCharacter
  (params (Index :type Integer) (SpawnTransform :type Transform))
  (bind _returnvalue (Game|SpawnActorfromClass "/Game/Blueprints/BP_Character_Sample.BP_Character_Sample_C" SpawnTransform "Undefined" "MultiplyWithRoot" self 0))
  (Pawn|Possess (Game|GetPlayerController Index) _returnvalue)
  (Default|InitPlayer (Variables|Reference|GetPSRef) Index))

(fn StartQuest
  (bind _returnvalue (Game|SpawnActorfromClass "/Game/Blueprints/BP_Quest_Sample.BP_Quest_Sample_C" (Math|Transform|MakeTransform "0, 0, 0") "Undefined" "MultiplyWithRoot" 0 0))
  (Variables|Reference|SetQuest _returnvalue)
  (Variables|/Game/Blueprints/Gamemode/BP_GS.BP_GS_C|SetbIsRunning (Variables|Reference|GetGSRef) true))