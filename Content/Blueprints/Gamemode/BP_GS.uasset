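; Game state Blueprint that drives the timed loop between battle quest stages and market breaks.
; During battle, Tick advances game and quest timers; when quest time hits its limit, the stage increments and battle pauses, or the Result level opens past the final stage.
; Outside battle, Tick calls SpawnMarket on GMRef every frame and counts market time until ResumeGameTime destroys the market.
; Timer and stage changes are pushed to the main HUD widget.
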(event Custom|ResumeGameTime
  ;[0 0 0] BP_Market) DestroyActor(); ResumeGameTime();
  (Default|DestroyMarket (Variables|Default|GetGMRef))
  (Variables|Default|SetbIsInBattle true)
  (Variables|Default|SetCurrentMarketTime 0.0))

(event EventTick
  (params (DeltaSeconds :type Float%20%28single-precision%29))
  (if (Variables|Default|GetbIsInBattle)
    (Utilities|FlowControl|Sequence
      (:then_0
        (CallFunction|SetGameTime))
      (:then_1
        (CallFunction|SetQuestTime)
        (CallFunction|ResetQuestTime)))
    (else
      (Default|SpawnMarket (Variables|Default|GetGMRef))
      (CallFunction|SetMarketTime))))

(fn ConstructionScript)

(fn SetGameTime
  (Variables|Default|SetCurrentGameTime (+ (Variables|Default|GetCurrentGameTime) (Utilities|Time|GetWorldDeltaSeconds)))
  (Default|SetGameTimeText (Variables|Default|GetUMGGameMainRef) (Variables|Default|GetCurrentGameTime)))

(fn SetMarketTime
  (Variables|Default|SetCurrentMarketTime (+ (Variables|Default|GetCurrentMarketTime) (Utilities|Time|GetWorldDeltaSeconds)))
  (Default|SetMarketTimeText (Variables|Default|GetUMGGameMainRef) (Variables|Default|GetCurrentMarketTime)))

(fn SetQuestTime
  (Variables|Default|SetCurrentQuestTime (+ (Variables|Default|GetCurrentQuestTime) (Utilities|Time|GetWorldDeltaSeconds)))
  (Default|SetQuestTimeText (Variables|Default|GetUMGGameMainRef) (Variables|Default|GetCurrentQuestTime)))

(fn ResetQuestTime
  (if (>= (Variables|Default|GetCurrentQuestTime) (Variables|Default|GetMaxQuestTime))
    (Variables|Default|SetCurrentQuestTime 0.0)
    (CallFunction|SetQuestStage)
    (Variables|Default|SetbIsInBattle false)))

(fn EndGame
  (if (> (Variables|Default|GetCurrentQuestStage) (Variables|Default|GetMaxQuestStage))
    (Game|OpenLevel(byName) "Result")))

(fn SetQuestStage
  (bind _output_get (Variables|Default|SetCurrentQuestStage (+ (Variables|Default|GetCurrentQuestStage) 1)))
  (Default|SetQuestStageText (Variables|Default|GetUMGGameMainRef) _output_get)
  (CallFunction|EndGame))