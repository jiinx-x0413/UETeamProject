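; BP_PC_Sample is a player controller for the game level that assigns the player's index and provides debug hotkeys.
; SetPlayerIndex, noted as called on Post Login, retries on a short delay until BP_PS is available, then copies the GameInstance's index to PlayerState and controller.
; T triggers EndGame on BP_GM_Game.
; M pops the market inventory, finding and caching BP_Market_Sample when the reference is invalid.
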(event Custom|SetPlayerIndex
  ;[0 0 0] SetPlayerIndex on Post Login :: Game Level
  (bind _asbp_ps (Utilities|Casting|CastToBP_PS (Variables|GetPlayerState))
    (:then
      (bind _asbp_gi (Utilities|Casting|CastToBP_GI (Game|GetGameInstance)))
      (bind _output_get (Variables|/Game/Blueprints/Gamemode/BP_PS.BP_PS_C|SetPlayerIndex _asbp_ps (Variables|/Game/Blueprints/Gamemode/BP_GI.BP_GI_C|GetPlayerIndex _asbp_gi)))
      (Variables|Default|SetPlayerIndex _output_get)
      (Development|PrintString (Utilities|String|ToString(Integer) _output_get) true true "(R=1.000000,G=0.780512,B=0.000000,A=1.000000)" 2e+01))
    (:CastFailed
      (Utilities|FlowControl|Delay 0.1)
      (CallFunction|SetPlayerIndex))))

(event Input|KeyboardEvents|T
  (params (Key :type Key%20Structure :default "None"))
  ;[1 1 1] debug :: endgame
  (:Pressed
    (bind _asbp_gm_game (Utilities|Casting|CastToBP_GM_Game (Game|GetGameMode)))
    (Default|EndGame _asbp_gm_game)))

(event Input|KeyboardEvents|M
  (params (Key :type Key%20Structure :default "None"))
  ;[1 1 1] debug::market inventory popup
  (:Pressed
    (Utilities|IsValid (Variables|Default|GetMarketRef)
      (:Is%20Valid
        (Default|PopMarketInventory (Variables|Default|GetMarketRef)))
      (:Is%20Not%20Valid
        (bind _returnvalue (Actor|GetActorOfClass "/Game/Blueprints/Game/Market/BP_Market_Sample.BP_Market_Sample_C"))
        (bind _output_get (Variables|Default|SetMarketRef _returnvalue))
        (Default|PopMarketInventory _output_get)))))

(fn ConstructionScript)