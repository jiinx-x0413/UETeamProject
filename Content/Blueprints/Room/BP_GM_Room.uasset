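; Room lobby game mode that tracks joined players, their names, ready states and character picks.
; PostLogin registers each controller, assigns its PlayerState index and adds 5 as the unselected character value.
; Events relay ready changes, new selection slots and character images to every BP_PC_Room, backfilling existing players' slots for newcomers.
; The CharacterSelection OnRep copies the selection array into each controller.
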(event Custom|SetAllPlayersReady
  (params (PlayerIndex :type Integer) (IsReady :type Boolean))
  ;[0 0 0] set player ready
  (for _array_element (Variables|Default|GetPCArray)
    (bind _asbp_pc_room (Utilities|Casting|CastToBP_PC_Room _array_element))
    (Default|SetPlayerReadyWidget _asbp_pc_room PlayerIndex IsReady)))

(event Custom|SetCharacterSelectionSlot
  (params (PlayerIndex :type Integer) (PlayerName :type String))
  ;[0 0 0] CharacterSelection
  (Development|PrintString (Utilities|String|Append (Utilities|String|ToString(Integer) PlayerIndex) "의 이름 : " PlayerName) true true "(R=0.608944,G=0.000000,B=1.000000,A=1.000000)" 2e+01)
  (for (_array_element _array_index) (Variables|Default|GetPCArray)
    ;;[0 0 0] Add pre Player select to New Player Widget
    (if (!= _array_index PlayerIndex)
      (CallFunction|AddPlayerSelectImage (Utilities|Array|Get(acopy) (Variables|Default|GetPCArray) PlayerIndex) _array_index))
    ;;[0 0 0] add New Player to All
    (CallFunction|AddPlayerSelectImage _array_element PlayerIndex)))

(event Custom|AddPlayerSelectImage
  (params (TargetPC :type Player%20Controller%20Object%20Reference) (NewPlayerIndex :type Integer))
  (bind _characterselection (Variables|Default|GetCharacterSelection))
  (bind _output (Utilities|Array|Get(acopy) _characterselection NewPlayerIndex))
  ;[0 0 0] CharacterSelection
  (bind _asbp_pc_room (Utilities|Casting|CastToBP_PC_Room TargetPC))
  (Default|ResAddPlayerSelectImage _asbp_pc_room NewPlayerIndex (Utilities|Array|Get(acopy) (Variables|Default|GetPlayerNameArray) NewPlayerIndex))
  ;;[0 0 0] Init Image
  (if (< _output 5)
    (Default|ResSetPlayerCharacterImage _asbp_pc_room NewPlayerIndex _output)))

(event Custom|SetPlayerSelectImageForAll
  (params (PlayerIndex :type Integer) (CharacterSelection :type Integer))
  ;[0 0 0] CharacterSelection
  (for _array_element (Variables|Default|GetPCArray)
    (bind _asbp_pc_room (Utilities|Casting|CastToBP_PC_Room _array_element))
    (Default|ResSetPlayerCharacterImage _asbp_pc_room PlayerIndex CharacterSelection)))

(event EventPostLogin
  (params (NewPlayer :type Player%20Controller%20Object%20Reference))
  (bind _returnvalue (Utilities|Array|Add (Variables|Default|GetPCArray) NewPlayer))
  (Utilities|Array|Add (Variables|Default|GetCharacterSelection) 5)
  ;[1 1 1] ps -> playerIndex
  (bind _asbp_ps (Utilities|Casting|CastToBP_PS (Variables|/Script/Engine.Controller|GetPlayerState NewPlayer)))
  (bind _output_get (Variables|/Game/Blueprints/Gamemode/BP_PS.BP_PS_C|SetPlayerIndex _asbp_ps _returnvalue))
  (bind _asbp_pc_room (Utilities|Casting|CastToBP_PC_Room NewPlayer))
  (Default|Init _asbp_pc_room _output_get))

(fn ConstructionScript)

(fn SelectCharacter
  (params (PlayerIndex :type Integer) (CharacterIndex :type Integer))
  (Utilities|Array|SetArrayElem (Variables|Default|GetCharacterSelection) PlayerIndex CharacterIndex))

(fn OnRepCharacterSelection
  (for _array_element (Variables|Default|GetPCArray)
    (bind _asbp_pc_room (Utilities|Casting|CastToBP_PC_Room _array_element))
    (Variables|/Game/Blueprints/Room/BP_PC_Room.BP_PC_Room_C|SetCharacterSelection _asbp_pc_room (Variables|Default|GetCharacterSelection))))

(fn SetCharacterImage)

(fn SetPlayerName
  (params (PlayerName :type String))
  (Utilities|Array|Add (Variables|Default|GetPlayerNameArray) PlayerName))

(fn OnRepPlayerNameArray)