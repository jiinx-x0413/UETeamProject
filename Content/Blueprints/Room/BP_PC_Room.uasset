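; Player controller for the pre-game room, handling character selection, ready state and game start.
; It creates the WBP_Room widget and tints player ready indicators green or white.
; Req_ events pass ready and selection changes to BP_GM_Room, while a Res_ event receives the selection data back.
; When all controllers are ready, the ready check copies selections to BP_GI and transitions to the Game level.
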(event Custom|Req_SelectCharacter
  (params (PlayerIndex :type Integer) (CharacterIndex :type Integer))
  (bind _asbp_gm_room (Utilities|Casting|CastToBP_GM_Room (Game|GetGameMode)))
  (Default|SelectCharacter _asbp_gm_room PlayerIndex CharacterIndex))

(event Custom|InitUI
  (bind _returnvalue (UserInterface|CreateWidget "/Game/Blueprints/Room/WBP_Room.WBP_Room_C"))
  (bind _output_get (Variables|Default|SetUIRoomRef _returnvalue))
  (UserInterface|Viewport|AddtoViewport _output_get 0))

(event Custom|Req_GetCharacterSelection
  (bind _asbp_gm_room (Utilities|Casting|CastToBP_GM_Room (Game|GetGameMode)))
  (CallFunction|ResGetCharacterSelection (Variables|/Game/Blueprints/Room/BP_GM_Room.BP_GM_Room_C|GetCharacterSelection _asbp_gm_room)))

(event Custom|Res_GetCharacterSelection
  (params (CharacterSelection :type Array%20of%20Integers))
  (Variables|Default|SetCharacterSelection CharacterSelection))

(event Custom|Req_CheckReady
  ;[0 0 0] Start Game
  (bind _asbp_gm_room (Utilities|Casting|CastToBP_GM_Room (Game|GetGameMode)))
  (Variables|/Game/Blueprints/Room/BP_GM_Room.BP_GM_Room_C|SetCountReady _asbp_gm_room 0)
  (for _array_element (Variables|/Game/Blueprints/Room/BP_GM_Room.BP_GM_Room_C|GetPCArray _asbp_gm_room)
    (bind _asbp_pc_room (Utilities|Casting|CastToBP_PC_Room _array_element))
    (if (Variables|BP_PC_Room_C|GetIsReady _asbp_pc_room)
      (Math|Integer|IncrementInt (Variables|/Game/Blueprints/Room/BP_GM_Room.BP_GM_Room_C|GetCountReady _asbp_gm_room))))
  (if (>= (Variables|/Game/Blueprints/Room/BP_GM_Room.BP_GM_Room_C|GetCountReady _asbp_gm_room) (Utilities|Array|Length (Variables|/Game/Blueprints/Room/BP_GM_Room.BP_GM_Room_C|GetPCArray _asbp_gm_room)))
    (bind _asbp_gi (Utilities|Casting|CastToBP_GI (Game|GetGameInstance)))
    (Variables|/Game/Blueprints/Gamemode/BP_GI.BP_GI_C|SetCharacterSelection _asbp_gi (Variables|/Game/Blueprints/Room/BP_GM_Room.BP_GM_Room_C|GetCharacterSelection _asbp_gm_room))
    (Default|LevelTransition _asbp_gi "Game")))

(event Custom|Req_SetReady
  (params (PlayerIndex :type Integer) (IsReady :type Boolean))
  ;[0 0 0] Set Ready
  (bind _output_get (Variables|Default|SetIsReady IsReady))
  ;;[1 1 1] BP_GM_Room
  (bind _asbp_gm_room (Utilities|Casting|CastToBP_GM_Room (Game|GetGameMode)))
  (Default|SetAllPlayersReady _asbp_gm_room PlayerIndex _output_get))

(event Custom|SetPlayerReadyWidget
  (params (Selection :type Integer) (Condition :type Boolean))
  ;[0 0 0] Set Ready
  (if Condition
    (Default|SetPlayerReady (Variables|Default|GetUIRoomRef) Selection "(R=0.296673,G=1.000000,B=0.277561,A=1.000000)")
    (else
      (Default|SetPlayerReady (Variables|Default|GetUIRoomRef) Selection "(R=1.000000,G=1.000000,B=1.000000,A=1.000000)"))))

(fn ConstructionScript)