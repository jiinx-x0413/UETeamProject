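; Sample player controller Blueprint that binds debug-style hotkeys for ending the match and opening the market.
; Pressing T casts the game mode to BP_GM_Ingame and calls EndGame.
; Pressing M pops the market inventory on a BP_Market_Sample actor, which it looks up in the level and caches on first use.
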(event Input|KeyboardEvents|T
  (params (Key :type Key%20Structure :default "None"))
  (:Pressed
    (bind _asbp_gm_ingame (Utilities|Casting|CastToBP_GM_Ingame (Game|GetGameMode)))
    (Default|EndGame _asbp_gm_ingame)))

(event Input|KeyboardEvents|M
  (params (Key :type Key%20Structure :default "None"))
  ;[0 0 0] market inventory popup
  (:Pressed
    (Utilities|IsValid (Variables|Default|GetMarketRef)
      (:Is%20Valid
        (Default|PopMarketInventory (Variables|Default|GetMarketRef)))
      (:Is%20Not%20Valid
        (bind _returnvalue (Actor|GetActorOfClass "/Game/Blueprints/Market/BP_Market_Sample.BP_Market_Sample_C"))
        (bind _output_get (Variables|Default|SetMarketRef _returnvalue))
        (Default|PopMarketInventory _output_get)))))

(fn ConstructionScript)